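; DeathTrigger is an overlap volume that ends a two-player physics-ball match when a ball enters it.
; It reads the ball's PlayerIndex, declares the other player the winner on screen and through a flag on the HUD, then destroys the ball.
; A Gameover flag blocks further wins, and a three-second timer calls RestartLevel, which reloads the current level by name.
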(event EventBeginPlay)

(event EventActorBeginOverlap
  (params (OtherActor :type Actor%20Object%20Reference))
  (if (not (Variables|Default|Getgameover))
    (bind _ashud (Utilities|Casting|CastToHUD (HUD|GetHUD (Game|GetPlayerController 0))))
    (bind _asphysics_ball_bp (Utilities|Casting|CastToPhysicsBallBP OtherActor))
    (if (== (Variables|/Game/RollingBP/Blueprints/PhysicsBallBP.PhysicsBallBP_C|GetPlayerIndex _asphysics_ball_bp) 0)
      (Development|PrintText "Player 2 WINS!!")
      (Variables|/Game/Blueprints/HUD.HUD_C|SetShowP2Win _ashud true)
      (Actor|DestroyActor _asphysics_ball_bp :!label _label)
      (Utilities|Time|SetTimerbyFunctionName 0 "RestartLevel" 3.0)
      (Variables|Default|Setgameover true)
      (elif (== (Variables|/Game/RollingBP/Blueprints/PhysicsBallBP.PhysicsBallBP_C|GetPlayerIndex _asphysics_ball_bp) 1)
        (Development|PrintText "Player 1 WINS!!!")
        (Variables|/Game/Blueprints/HUD.HUD_C|SetShowP1Win _ashud true)
        (goto _label)))))

(event EventTick
  (params (DeltaSeconds :type Float%20%28single-precision%29)))

(fn ConstructionScript)

(fn RestartLevel
  (bind _returnvalue (Game|GetCurrentLevelName true))
  (Game|OpenLevel(byName) (Utilities|String|StringToName _returnvalue)))