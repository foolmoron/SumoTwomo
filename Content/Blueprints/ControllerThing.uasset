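; ControllerThing is an input-routing Blueprint for a two-player game with left and right controls per player.
; It mirrors each player's left and right action presses and releases into LeftDown and RightDown flags on Player1 and Player2.
; On BeginPlay it caches the cast HUD, and any press clears the HUD's ShowStarting flag.
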(event EventBeginPlay)

(event EventActorBeginOverlap
  (params (OtherActor :type Actor%20Object%20Reference)))

(event EventTick
  (params (DeltaSeconds :type Float%20%28single-precision%29)))

(event EventBeginPlay
  (bind _ashud (Utilities|Casting|CastToHUD (HUD|GetHUD (Game|GetPlayerController 0)))))

(event Input|ActionEvents|InputActionP1Left
  (params (Key :type Key%20Structure :default "AnyKey"))
  (:Pressed
    (Variables|/Game/RollingBP/Blueprints/PhysicsBallBP.PhysicsBallBP_C|SetLeftDown (Variables|Default|GetPlayer1) true)
    (Variables|/Game/Blueprints/HUD.HUD_C|SetShowStarting (stale EventBeginPlay _ashud) false))
  (:Released
    (Variables|/Game/RollingBP/Blueprints/PhysicsBallBP.PhysicsBallBP_C|SetLeftDown (Variables|Default|GetPlayer1) false)))

(event Input|ActionEvents|InputActionP1Right
  (params (Key :type Key%20Structure :default "AnyKey"))
  (:Pressed
    (Variables|/Game/RollingBP/Blueprints/PhysicsBallBP.PhysicsBallBP_C|SetRightDown (Variables|Default|GetPlayer1) true)
    (Variables|/Game/Blueprints/HUD.HUD_C|SetShowStarting (stale EventBeginPlay _ashud) false))
  (:Released
    (Variables|/Game/RollingBP/Blueprints/PhysicsBallBP.PhysicsBallBP_C|SetRightDown (Variables|Default|GetPlayer1) false)))

(event Input|ActionEvents|InputActionP2Left
  (params (Key :type Key%20Structure :default "AnyKey"))
  (:Pressed
    (Variables|/Game/RollingBP/Blueprints/PhysicsBallBP.PhysicsBallBP_C|SetLeftDown (Variables|Default|GetPlayer2) true)
    (Variables|/Game/Blueprints/HUD.HUD_C|SetShowStarting (stale EventBeginPlay _ashud) false))
  (:Released
    (Variables|/Game/RollingBP/Blueprints/PhysicsBallBP.PhysicsBallBP_C|SetLeftDown (Variables|Default|GetPlayer2) false)))

(event Input|ActionEvents|InputActionP2Right
  (params (Key :type Key%20Structure :default "AnyKey"))
  (:Pressed
    (Variables|/Game/RollingBP/Blueprints/PhysicsBallBP.PhysicsBallBP_C|SetRightDown (Variables|Default|GetPlayer2) true)
    (Variables|/Game/Blueprints/HUD.HUD_C|SetShowStarting (stale EventBeginPlay _ashud) false))
  (:Released
    (Variables|/Game/RollingBP/Blueprints/PhysicsBallBP.PhysicsBallBP_C|SetRightDown (Variables|Default|GetPlayer2) false)))

(fn ConstructionScript)