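; HUD for a two-player Twomo game (Ludum Dare 34) that draws the start screen and winner banners.
; DrawHUD checks ShowStarting, then ShowP1Win, then ShowP2Win to show controls, credit and title, or the winning player's image.
; Each banner is stacked in a loop of shrinking, increasingly opaque copies with time-cycled HSV tints, creating an animated rainbow glow anchored to the bottom center of the viewport.
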(event EventBeginPlay)

(event EventActorBeginOverlap
  (params (OtherActor :type Actor%20Object%20Reference)))

(event EventTick
  (params (DeltaSeconds :type Float%20%28single-precision%29)))

(event EventDrawHUD
  (params (SizeX :type Integer) (SizeY :type Integer))
  (bind _returnvalue (Game|GetPlayerController 0))
  (bind (_sizex _sizey) (HUD|GetViewportSize _returnvalue))
  (bind _returnvalue_2 (/ _sizex 2))
  (if (Variables|Default|GetShowStarting)
    (HUD|DrawText "Twomo 1 
[A] - turn left 
[S] - turn right 
[A + S] - BOOST 
hold [A + S] - GROW" "(R=1.000000,G=1.000000,B=1.000000,A=1.000000)" 15.0 1e+02 "/Game/Blueprints/HUDFont.HUDFont" 1.0 false)
    (HUD|DrawText "Twomo 2 
[K] - turn left 
[L] - turn right 
[K + L] - BOOST 
hold [K + L] - GROW" "(R=1.000000,G=1.000000,B=1.000000,A=1.000000)" (Math|Conversions|ToFloat(Integer) (+ _sizex -410)) 1e+02 "/Game/Blueprints/HUDFont.HUDFont" 1.0 false)
    (for _index (range 0 20)
      (Canvas|DrawTexture "/Game/Rolling/Materials/title.title" (Math|Conversions|ToFloat(Integer) (+ _returnvalue_2 (+ (* (- 20 _index) -3) -420))) (Math|Conversions|ToFloat(Integer) (+ _sizey (+ (* (- 20 _index) -3) -220))) (Math|Conversions|ToFloat(Integer) (+ (* (- 20 _index) 6) 800)) (Math|Conversions|ToFloat(Integer) (+ (* (- 20 _index) 6) 200)) 0.0 0.0 1.0 1.0 (Class|KismetMathLibrary|HSVtoRGB (Math|Conversions|ToFloat(Integer) (Math|Integer|%(Integer) (+ (* _index 30) (Math|Float|Truncate (* (Utilities|Time|GetGameTimeinSeconds) 1.5e+02))) 256)) 1.0 0.7 (* (Math|Conversions|ToFloat(Integer) _index) 0.05)))
      (HUD|DrawText "by @foolmoron for Ludum Dare 34" "(R=1.000000,G=1.000000,B=1.000000,A=1.000000)" (+ -3.5e+02 (Math|Conversions|ToFloat(Integer) _returnvalue_2)) (+ -7e+01 (Math|Conversions|ToFloat(Integer) _sizey)) "/Game/Blueprints/HUDFont.HUDFont" 1.0 false))
    (elif (Variables|Default|GetShowP1Win)
      (for _index_2 (range 0 20)
        (Canvas|DrawTexture "/Game/Rolling/Materials/twomo1.twomo1" (Math|Conversions|ToFloat(Integer) (+ _returnvalue_2 (+ (* (- 20 _index_2) -3) -420))) (Math|Conversions|ToFloat(Integer) (+ _sizey (+ (* (- 20 _index_2) -3) -220))) (Math|Conversions|ToFloat(Integer) (+ (* (- 20 _index_2) 6) 800)) (Math|Conversions|ToFloat(Integer) (+ (* (- 20 _index_2) 6) 200)) 0.0 0.0 1.0 1.0 (Class|KismetMathLibrary|HSVtoRGB (Math|Conversions|ToFloat(Integer) (Math|Integer|%(Integer) (+ (* _index_2 30) (Math|Float|Truncate (* (Utilities|Time|GetGameTimeinSeconds) 1.5e+02))) 256)) 1.0 0.7 (* (Math|Conversions|ToFloat(Integer) _index_2) 0.05))))
      (elif (Variables|Default|GetShowP2Win)
        (for _index_3 (range 0 20)
          (Canvas|DrawTexture "/Game/Rolling/Materials/twomo2.twomo2" (Math|Conversions|ToFloat(Integer) (+ _returnvalue_2 (+ (* (- 20 _index_3) -3) -420))) (Math|Conversions|ToFloat(Integer) (+ _sizey (+ (* (- 20 _index_3) -3) -220))) (Math|Conversions|ToFloat(Integer) (+ (* (- 20 _index_3) 6) 800)) (Math|Conversions|ToFloat(Integer) (+ (* (- 20 _index_3) 6) 200)) 0.0 0.0 1.0 1.0 (Class|KismetMathLibrary|HSVtoRGB (Math|Conversions|ToFloat(Integer) (Math|Integer|%(Integer) (+ (* _index_3 30) (Math|Float|Truncate (* (Utilities|Time|GetGameTimeinSeconds) 1.5e+02))) 256)) 1.0 0.7 (* (Math|Conversions|ToFloat(Integer) _index_3) 0.05))))))))

(fn ConstructionScript)